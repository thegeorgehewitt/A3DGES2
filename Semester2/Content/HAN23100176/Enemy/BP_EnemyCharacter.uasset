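; BP_EnemyCharacter is a melee enemy that chases pawns it senses and punches them.
; PawnSensing sightings trigger FollowPlayer, which uses AI MoveTo to approach the seen pawn.
; On arrival, a CanAttack flag gates the punch montage until it completes.
; HitPlayer runs as the montage starts, waits briefly, then applies fixed damage to every actor overlapping its Box, with no target filter.
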(event `self.PawnSensing.OnSeePawn`
  (params (Pawn :type "Pawn Object Reference"))
  (set `self.IsSeeingPlayer` true)
  (`self.FollowPlayer`))

(event `FollowPlayer`
  (if (`self.IsSeeingPlayer`)
    (`|AIMoveTo` self (0.0 0.0 0.0) (stale `self.PawnSensing.OnSeePawn` Pawn) 70.0
      (:`OnSuccess`
        (if (`self.CanAttack`)
          (set `self.CanAttack` false)
          (`|PlayMontage` (`self.Mesh`) "/Game/HAN23100176/Enemy/Animations/AM_Punch.AM_Punch"
            (:`then`
              (`self.HitPlayer`))
            (:`OnCompleted`
              (set `self.CanAttack` true))))))
    (else
      (set `self.IsSeeingPlayer` false))))

(event `HitPlayer`
  (`KismetSystemLibrary.Delay` 0.2)
  (for _array_element (`PrimitiveComponent.GetOverlappingActors` (`self.Box`) null)
    (`GameplayStatics.ApplyDamage` _array_element 5.0)))

(fn `UserConstructionScript`)