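; GM_Collect is a game mode for a timed item-collection game.
; On BeginPlay it runs the parent logic, then spawns a BP_PickupManager for two pickups and a BP_TimeManager with a ten-second timer, passing itself to both.
; Its WinCollected event prints a completion message with an empty seconds value, flags all items as collected and calls CanEndGame.
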(event `InitPickups`
  (bind _returnvalue (`|SpawnActorFromClass` "/Game/HAN23100176/Gameplay/BP_PickupManager.BP_PickupManager_C" (`KismetMathLibrary.MakeTransform` (0.0 0.0 0.0)) "Undefined" "OverrideRootScale" null null))
  (`/Game/HAN23100176/Gameplay/BP_PickupManager.InitPickups` _returnvalue self 2))

(event `/Game/HAN23100176/Gameplay/Interfaces/BPI_WinConditions.Win_Collected`
  (params (WinningTeam :type "/Game/HAN23100176/Gameplay/E_Teams Enum" :default "NewEnumerator0"))
  (`KismetSystemLibrary.PrintString` (`KismetStringLibrary.Concat_StrStr` " All collected in " "" " seconds"))
  (set `self.HaveAllItemsCollected` true)
  (`self.CanEndGame`))

(event `self.ReceiveBeginPlay`
  (`parent.ReceiveBeginPlay`)
  (`KismetSystemLibrary.PrintString` "GM_Collect Running")
  (`self.InitPickups`)
  (`self.InitTimer`))

(event `InitTimer`
  (bind _returnvalue (`|SpawnActorFromClass` "/Game/HAN23100176/Gameplay/BP_TimeManager.BP_TimeManager_C" (`KismetMathLibrary.MakeTransform` (0.0 0.0 0.0)) "Undefined" "OverrideRootScale" null null))
  (`/Game/HAN23100176/Gameplay/BP_TimeManager.InitTimer` _returnvalue 10.0 self))

(fn `UserConstructionScript`)