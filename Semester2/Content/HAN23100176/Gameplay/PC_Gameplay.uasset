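; PC_Gameplay is the gameplay player controller, holding each player's data, including team ID, behind simple setters and getters.
; SetPlayerData replaces the whole PlayerData struct, while SetTeam updates only its TeamID member.
; Pressing M calls RemovePlayers and then opens the main menu map.
; BeginPlay prints a debug message to show the controller is running.
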(event `self.ReceiveBeginPlay`
  (`KismetSystemLibrary.PrintString` "PC_Gameplay Running"))

(event `Key|M`
  (params (Key :type "Key Structure"))
  (:`Pressed`
    (`/Game/HAN23100176/Gameplay/BPL_Gameplay.RemovePlayers`)
    (`GameplayStatics.OpenLevel` "MainMenu_Map")))

(event `/Game/HAN23100176/Gameplay/BPI_PlayerData.SetTeam`
  (params (TeamID :type "/Game/HAN23100176/Gameplay/E_Teams Enum" :default "NewEnumerator0"))
  (setmembers `/Game/HAN23100176/Gameplay/S_PlayerData` :`StructRef` (`self.Player Data`) :`TeamID` TeamID))

(event `/Game/HAN23100176/Gameplay/BPI_PlayerData.SetPlayerData`
  (params (PlayerData :type "/Game/HAN23100176/Gameplay/S_PlayerData Structure"))
  (set `self.Player Data` PlayerData))

(fn `GetPlayerData`
  (returns (PlayerData :type "/Game/HAN23100176/Gameplay/S_PlayerData Structure"))
  (return (`self.Player Data`)))

(fn `GetTeam`
  (returns (TeamID :type "/Game/HAN23100176/Gameplay/E_Teams Enum"))
  (return (`.TeamID_13_7275F7AE4C2E83F063AD92B2A0A26EA5` (break `/Game/HAN23100176/Gameplay/S_PlayerData` (`self.Player Data`)))))

(fn `UserConstructionScript`)