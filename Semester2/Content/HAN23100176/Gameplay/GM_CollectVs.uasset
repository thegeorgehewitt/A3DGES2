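; Game mode for a collection-based versus match, where collecting every item counts toward ending the game.
; On BeginPlay it runs the parent logic, then spawns a BP_PickupManager at the world origin and initializes it with a reference to itself.
; WinCollected flags that all items are collected and calls CanEndGame to check for the end of the match.
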(event `InitPickups`
  (bind _returnvalue (`|SpawnActorFromClass` "/Game/HAN23100176/Gameplay/BP_PickupManager.BP_PickupManager_C" (`KismetMathLibrary.MakeTransform` (0.0 0.0 0.0)) "Undefined" "OverrideRootScale" null null))
  (`/Game/HAN23100176/Gameplay/BP_PickupManager.InitPickups` _returnvalue self))

(event `/Game/HAN23100176/Gameplay/BPI_WinConditions.Win_Collected`
  (set `self.HaveAllItemsCollected` true)
  (`self.CanEndGame`))

(event `self.ReceiveBeginPlay`
  (`parent.ReceiveBeginPlay`)
  (`KismetSystemLibrary.PrintString` "GM_Collect Running")
  (`self.InitPickups`))

(fn `UserConstructionScript`)