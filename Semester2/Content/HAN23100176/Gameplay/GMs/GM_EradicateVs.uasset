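; Game mode for Eradicate Versus, where a match can end with a winning team once enemies are killed, or in game over when all players die.
; On BeginPlay it spawns an enemy manager with spawners and a time manager running the match timer, passing itself to both.
; Player deaths shrink the player list until empty; both outcomes call CanEndGame.
; State changes drive the timed start screen and delayed EndGame.
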(event `self.ReceiveBeginPlay`
  (`parent.ReceiveBeginPlay`)
  (`KismetSystemLibrary.PrintString` "GM Eradicate Versus Running")
  (`self.InitEnemyManager`)
  (`self.InitTimer`)
  (add `self.OnPlayerDied` (delegate `PlayerDied`)))

(event `PlayerDied` :!signature `self.OnPlayerDied`
  (params (DeadPlayer :type "/Game/HAN23100176/Characters/Paladin/BP_ThirdPersonCharacter Object Reference"))
  (bind _allplayers (`self.AllPlayers`))
  (bind _aspc_gameplay (cast `/Game/HAN23100176/Gameplay/PC_Gameplay` (`Pawn.GetController` DeadPlayer)))
  (`KismetArrayLibrary.Array_RemoveItem` _allplayers _aspc_gameplay)
  (if (== (`KismetArrayLibrary.Array_Length` _allplayers) 0)
    (`/Game/HAN23100176/Gameplay/Interfaces/BPI_WinConditions.Win_PlayersDead`)))

(event `InitEnemyManager`
  (bind _returnvalue (`|SpawnActorFromClass` "/Game/HAN23100176/Gameplay/EnemySystem/BP_EnemyManager.BP_EnemyManager_C" (`KismetMathLibrary.MakeTransform` (0.0 0.0 0.0)) "Undefined" "OverrideRootScale" null null))
  (`/Game/HAN23100176/Gameplay/EnemySystem/BP_EnemyManager.InitEnemySpawners` _returnvalue self 8))

(event `InitTimer`
  (bind _returnvalue (`|SpawnActorFromClass` "/Game/HAN23100176/Gameplay/TimeSystem/BP_TimeManager.BP_TimeManager_C" (`KismetMathLibrary.MakeTransform` (0.0 0.0 0.0)) "Undefined" "OverrideRootScale" null null))
  (`/Game/HAN23100176/Gameplay/TimeSystem/BP_TimeManager.InitTimer` _returnvalue 240.0 self))

(event `/Game/HAN23100176/Gameplay/Interfaces/BPI_WinConditions.Win_EnemiesKilled`
  (params (WinningTeam :type "/Game/HAN23100176/Gameplay/E_Teams Enum" :default "NewEnumerator0"))
  (`KismetSystemLibrary.PrintString` (`KismetStringLibrary.Concat_StrStr` (`|GetEnumeratorNameAsString` WinningTeam) " wins!"))
  (set `self.AllEnemiesKilled` true)
  (`self.CanEndGame`))

(event `/Game/HAN23100176/Gameplay/Interfaces/BPI_WinConditions.Win_PlayersDead`
  (`KismetSystemLibrary.PrintString` "Game Over")
  (set `self.HaveAllPlayersDied` true)
  (`self.CanEndGame`))

(event `self.GameStateChanged`
  (params (CurrentGameState :type "/Game/HAN23100176/Gameplay/E_GameState Enum" :default "NewEnumerator0"))
  (switch `/Game/HAN23100176/Gameplay/E_GameState` CurrentGameState
    (:`NewEnumerator1`
      (`KismetSystemLibrary.PrintString` "Pre Game")
      (`/Game/HAN23100176/UI/WBP_StartScreen.SetUp` (`self.StartScreen`) "Eradicate Versus" (`self.PreGameTime`))
      (`KismetSystemLibrary.Delay` (`self.PreGameTime`))
      (`/Game/HAN23100176/Gameplay/GS_GameStateBase.UpdateState` (`self.MyGameState`) "NewEnumerator2"))
    (:`NewEnumerator2`
      (`KismetSystemLibrary.PrintString` "In Game"))
    (:`NewEnumerator3`
      (`KismetSystemLibrary.PrintString` "Post Game")
      (`KismetSystemLibrary.Delay` 3.0)
      (`self.EndGame`))))

(fn `UserConstructionScript`
  (`parent.UserConstructionScript`))