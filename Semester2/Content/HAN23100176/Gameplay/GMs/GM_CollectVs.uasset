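; Game mode for Collect Versus, a team-based pickup collection match.
; On BeginPlay it spawns pickup and time managers that reference it, while pre-game state shows a start screen, then initializes the versus UI and switches to in-game.
; WinCollected stores the winning team and scores, then, if the game can end, shows the death, timeout or win screen before ending.
; The level UI's time is set separately from the timer's length, and the two differ.
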(event `self.ReceiveBeginPlay`
  (`parent.ReceiveBeginPlay`)
  (`KismetSystemLibrary.PrintString` "GM Collect Versus Running")
  (`self.InitPickups`)
  (`self.InitTimer`))

(event `InitPickups`
  (bind _returnvalue (`|SpawnActorFromClass` "/Game/HAN23100176/Gameplay/PickupSystem/BP_PickupManager.BP_PickupManager_C" (`KismetMathLibrary.MakeTransform` (0.0 0.0 0.0)) "Undefined" "OverrideRootScale" null (`self.LevelUI`) null))
  (`/Game/HAN23100176/Gameplay/PickupSystem/BP_PickupManager.InitPickups` _returnvalue self 2))

(event `InitTimer`
  (bind _returnvalue (`|SpawnActorFromClass` "/Game/HAN23100176/Gameplay/TimeSystem/BP_TimeManager.BP_TimeManager_C" (`KismetMathLibrary.MakeTransform` (0.0 0.0 0.0)) "Undefined" "OverrideRootScale" null null))
  (`/Game/HAN23100176/Gameplay/TimeSystem/BP_TimeManager.InitTimer` _returnvalue 20.0 self))

(event `/Game/HAN23100176/Gameplay/Interfaces/BPI_WinConditions.Win_Collected`
  (params (WinningTeam :type "/Game/HAN23100176/Gameplay/E_Teams Enum" :default "NewEnumerator0") (TeamAScore :type Integer) (TeamBScore :type Integer))
  (set `self.Winning Team` WinningTeam)
  (set `self.Team AScore` TeamAScore)
  (set `self.Team BScore` TeamBScore)
  (`KismetSystemLibrary.PrintString` (`KismetStringLibrary.Concat_StrStr` (`|GetEnumeratorNameAsString` WinningTeam) " wins!"))
  (set `self.HaveAllItemsCollected` true)
  (bind _newparam (`self.CanEndGame`))
  (if _newparam
    (`KismetSystemLibrary.Delay` 1.0)
    (if (`self.HaveAllPlayersDied`)
      (`/Game/HAN23100176/UI/WBP_EndScreen.SetUp` (`self.EndScreen`) false "NewEnumerator0" 0 0 "All Players Died")
      (`Widget.SetVisibility` (`self.EndScreen`) "Visible" :!label _label)
      (`KismetSystemLibrary.Delay` 8.0)
      (`self.EndGame`)
      (elif (`self.HasTimeRunOut`)
        (`/Game/HAN23100176/UI/WBP_EndScreen.SetUp` (`self.EndScreen`) false "NewEnumerator0" 0 0 "Out of Time")
        (goto _label)
        (elif (`self.HaveAllItemsCollected`)
          (`/Game/HAN23100176/UI/WBP_EndScreen.SetUp` (`self.EndScreen`) true (`self.Winning Team`) (`self.Team AScore`) (`self.Team BScore`) "")
          (goto _label))))))

(event `self.GameStateChanged`
  (params (CurrentGameState :type "/Game/HAN23100176/Gameplay/E_GameState Enum" :default "NewEnumerator0"))
  (switch `/Game/HAN23100176/Gameplay/E_GameState` CurrentGameState
    (:`NewEnumerator1`
      (`KismetSystemLibrary.PrintString` "Pre Game")
      (`/Game/HAN23100176/UI/WBP_StartScreen.SetUp` (`self.StartScreen`) "Collect Versus" (`self.PreGameTime`))
      (`KismetSystemLibrary.Delay` (`self.PreGameTime`))
      (`/Game/HAN23100176/UI/WBP_SharedLevelUI.Initialize` (`self.LevelUI`) 60.0 true)
      (`/Game/HAN23100176/Gameplay/GS_GameStateBase.UpdateState` (`self.MyGameState`) "NewEnumerator2"))
    (:`NewEnumerator2`
      (`KismetSystemLibrary.PrintString` "In Game"))
    (:`NewEnumerator3`
      (`KismetSystemLibrary.PrintString` "Post Game"))))

(fn `UserConstructionScript`)