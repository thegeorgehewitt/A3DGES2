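; Game mode for Eradicate, a timed match won by killing all enemies and lost when every player dies or time runs out.
; On BeginPlay it spawns an enemy manager with its spawners and a time manager, and tracks player deaths to empty the player list.
; Win and death events set flags and call CanEndGame.
; Game state changes drive the start screen countdown, level UI and result screen before ending the game.
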(event `self.ReceiveBeginPlay`
  (`parent.ReceiveBeginPlay`)
  (`self.InitEnemyManager`)
  (`self.InitTimer`)
  (add `self.OnPlayerDied` (delegate `PlayerDied`)))

(event `PlayerDied` :!signature `self.OnPlayerDied`
  (params (DeadPlayer :type "/Game/HAN23100176/Characters/Paladin/BP_ThirdPersonCharacter Object Reference"))
  (bind _allplayers (`self.AllPlayers`))
  (bind _aspc_gameplay (cast `/Game/HAN23100176/Gameplay/PC_Gameplay` (`Pawn.GetController` DeadPlayer)))
  (`KismetArrayLibrary.Array_RemoveItem` _allplayers _aspc_gameplay)
  (if (== (`KismetArrayLibrary.Array_Length` _allplayers) 0)
    (`/Game/HAN23100176/Gameplay/Interfaces/BPI_WinConditions.Win_PlayersDead`)))

(event `InitEnemyManager`
  (bind _returnvalue (`|SpawnActorFromClass` "/Game/HAN23100176/Gameplay/EnemySystem/BP_EnemyManager.BP_EnemyManager_C" (`KismetMathLibrary.MakeTransform` (0.0 0.0 0.0)) "Undefined" "OverrideRootScale" null null null))
  (`/Game/HAN23100176/Gameplay/EnemySystem/BP_EnemyManager.InitEnemySpawners` _returnvalue self 4))

(event `InitTimer`
  (bind _returnvalue (`|SpawnActorFromClass` "/Game/HAN23100176/Gameplay/TimeSystem/BP_TimeManager.BP_TimeManager_C" (`KismetMathLibrary.MakeTransform` (0.0 0.0 0.0)) "Undefined" "OverrideRootScale" null null))
  (`/Game/HAN23100176/Gameplay/TimeSystem/BP_TimeManager.InitTimer` _returnvalue 63.0 self)
  (set `self.TimeManager` _returnvalue))

(event `/Game/HAN23100176/Gameplay/Interfaces/BPI_WinConditions.Win_EnemiesKilled`
  (params (WinningTeam :type "/Game/HAN23100176/Gameplay/E_Teams Enum" :default "NewEnumerator0") (TeamAScore :type Integer) (TeamBScore :type Integer))
  (set `self.AllEnemiesKilled` true)
  (`self.CanEndGame`))

(event `/Game/HAN23100176/Gameplay/Interfaces/BPI_WinConditions.Win_PlayersDead`
  (set `self.HaveAllPlayersDied` true)
  (`self.CanEndGame`))

(event `self.GameStateChanged`
  (params (CurrentGameState :type "/Game/HAN23100176/Gameplay/E_GameState Enum" :default "NewEnumerator0"))
  (switch `/Game/HAN23100176/Gameplay/E_GameState` CurrentGameState
    (:`NewEnumerator1`
      (`/Game/HAN23100176/UI/WBP_StartScreen.SetUp` (`self.StartScreen`) "Eradicate" (`self.PreGameTime`))
      (`KismetSystemLibrary.Delay` (`self.PreGameTime`))
      (`/Game/HAN23100176/UI/WBP_SharedLevelUI.Initialize` (`self.LevelUI`) 60.0 false)
      (`/Game/HAN23100176/Gameplay/GS_GameStateBase.UpdateState` (`self.MyGameState`) "NewEnumerator2"))
    (:`NewEnumerator3`
      (`KismetSystemLibrary.Delay` 1.0)
      (if (`self.HaveAllPlayersDied`)
        (`/Game/HAN23100176/UI/WBP_EndScreen.SetUp` (`self.EndScreen`) false "NewEnumerator0" 0 0 "All Players Died")
        (`Widget.SetVisibility` (`self.LevelUI`) "Hidden" :!label _label)
        (`Widget.SetVisibility` (`self.EndScreen`) "Visible")
        (`KismetSystemLibrary.Delay` 8.0)
        (`self.EndGame`)
        (elif (`self.HasTimeRunOut`)
          (`/Game/HAN23100176/UI/WBP_EndScreen.SetUp` (`self.EndScreen`) false "NewEnumerator0" 0 0 "Out of Time")
          (goto _label)
          (elif (`self.AllEnemiesKilled`)
            (bind _timeelapsed (`/Game/HAN23100176/Gameplay/TimeSystem/BP_TimeManager.GetTimeElapsed` (`self.TimeManager`)))
            (`/Game/HAN23100176/UI/WBP_EndScreen.SetUp` (`self.EndScreen`) true "NewEnumerator0" 0 0 (`KismetTextLibrary.Conv_StringToText` (`KismetStringLibrary.Concat_StrStr` "All enemies killed in " (`KismetStringLibrary.Conv_DoubleToString` _timeelapsed) " seconds")))
            (goto _label)))))))

(fn `UserConstructionScript`
  (`parent.UserConstructionScript`))