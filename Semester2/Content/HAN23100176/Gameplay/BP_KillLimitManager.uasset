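; Kill limit manager that tracks kills for two teams and triggers a win once either reaches the target.
; Init stores the game mode reference and target, then binds to the player-killed event of existing BP_ThirdPersonCharacter actors.
; UpdateKills credits the team opposite the one passed in and calls WinEnemiesKilledMessage on GMRef with that team when its count meets the target.
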(event `Init`
  (params (GMRef :type "GameModeBase Object Reference") (TargetKills :type Integer))
  (set `self.GMRef` GMRef)
  (set `self.Target Kills` TargetKills)
  (bind _outactors (`GameplayStatics.GetAllActorsOfClass` "/Game/ThirdPerson/Blueprints/BP_ThirdPersonCharacter.BP_ThirdPersonCharacter_C"))
  (add `/Game/ThirdPerson/Blueprints/BP_ThirdPersonCharacter.PlayerKilled` _outactors (`|CreateDelegate` :!event `UpdateKills`)))

(event `UpdateKills`
  (params (Team :type "/Game/HAN23100176/Gameplay/E_Teams Enum" :default "NewEnumerator0"))
  (switch `/Game/HAN23100176/Gameplay/E_Teams` Team
    (:`NewEnumerator1`
      (bind _result (`/Engine/EditorBlueprintResources/StandardMacros.IncrementInt` (`self.TeamBKills`))
        (:`  `
          (if (>= _result (`self.Target Kills`))
            (message `/Game/HAN23100176/Gameplay/BPI_WinConditions.Win_EnemiesKilled` (`self.GMRef`) "NewEnumerator2")))))
    (:`NewEnumerator2`
      (bind _result_2 (`/Engine/EditorBlueprintResources/StandardMacros.IncrementInt` (`self.TeamAKills`))
        (:`  `
          (if (>= _result_2 (`self.Target Kills`))
            (message `/Game/HAN23100176/Gameplay/BPI_WinConditions.Win_EnemiesKilled` (`self.GMRef`) "NewEnumerator1")))))))

(fn `UserConstructionScript`)