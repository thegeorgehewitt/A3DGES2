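; BP_EnemySpawner is a destructible spawner actor that places BP_EnemyCharacter enemies at random reachable navmesh points around itself.
; InitEnemies spawns an initial batch, then starts a looping timer on SpawnDelay for an event delegate.
; Each spawned enemy receives ManagerRef and is reported to that manager.
; AnyDamage reduces SpawnerHealth, and at zero or below the spawner notifies the manager and destroys itself.
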(event `SpawnEnemy`
  (bind _returnvalue (`|SpawnActorFromClass` "/Game/HAN23100176/Characters/Enemy/BP_EnemyCharacter.BP_EnemyCharacter_C" (`KismetMathLibrary.MakeTransform` (`NavigationSystemV1.K2_GetRandomReachablePointInRadius` (`self.K2_GetActorLocation`) 500.0 null null)) "AdjustIfPossibleButAlwaysSpawn" "OverrideRootScale" null (`self.ManagerRef`) null :!label _label))
  (`/Game/HAN23100176/Gameplay/BP_EnemyManager.EnemySpawned` (`self.ManagerRef`) _returnvalue))

(event `InitEnemies`
  (for _ (range 1 (+ (`self.InitialSpawnCount`) 1))
    (goto _label))
  (`KismetSystemLibrary.K2_SetTimerDelegate` (`|CreateDelegate` :!event `SpawnEnemy`) (`self.SpawnDelay`) true))

(event `self.ReceiveAnyDamage`
  (params (Damage :type "Float (single-precision)") (DamageType :type "DamageType Object Reference") (InstigatedBy :type "Controller Object Reference") (DamageCauser :type "Actor Object Reference"))
  (bind _output_get (set `self.SpawnerHealth` (- (`self.SpawnerHealth`) Damage)))
  (if (<= _output_get 0.0)
    (`/Game/HAN23100176/Gameplay/BP_EnemyManager.SpawnerDestroyed` (`self.ManagerRef`) self)
    (`self.K2_DestroyActor`)))

(fn `UserConstructionScript`)