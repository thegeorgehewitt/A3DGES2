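; BP_EnemySpawner is a destructible spawner that places BP_EnemyCharacter enemies at random reachable navmesh points nearby, with random yaw.
; InitEnemies spawns an initial batch, then creates a looping spawn timer that starts paused.
; A sphere overlap runs the timer only while a Player-tagged actor is in range.
; It reports each spawned enemy to ManagerRef and, when its health runs out, its own destruction before removing itself.
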(event `SpawnEnemy`
  (bind (_returnvalue_roll _returnvalue_pitch _returnvalue_yaw) (`KismetMathLibrary.BreakRotator` (`KismetMathLibrary.RandomRotator` false)))
  (bind _returnvalue (`|SpawnActorFromClass` "/Game/HAN23100176/Characters/Enemy/BP_EnemyCharacter.BP_EnemyCharacter_C" (`KismetMathLibrary.MakeTransform` (`NavigationSystemV1.K2_GetRandomReachablePointInRadius` (`self.K2_GetActorLocation`) 200.0 null null) (`KismetMathLibrary.MakeRotator` 0.0 0.0 _returnvalue_yaw)) "AdjustIfPossibleButDontSpawnIfColliding" "OverrideRootScale" null (`self.ManagerRef`) null :!label _label))
  (`/Engine/EditorBlueprintResources/StandardMacros.IsValid` _returnvalue
    (:`Is Valid`
      (`KismetSystemLibrary.PrintString` (`KismetSystemLibrary.GetDisplayName` _returnvalue))
      (`/Game/HAN23100176/Gameplay/EnemySystem/BP_EnemyManager.EnemySpawned` (`self.ManagerRef`) _returnvalue))
    (:`Is Not Valid`
      (`KismetSystemLibrary.PrintString` "failed"))))

(event `InitEnemies`
  (`KismetSystemLibrary.PrintString` "init enemies")
  (for _index (range (`self.InitialSpawnCount`))
    (`KismetSystemLibrary.PrintString` (`KismetStringLibrary.Conv_IntToString` _index))
    (goto _label))
  (bind _returnvalue (`KismetSystemLibrary.K2_SetTimerDelegate` (`|CreateDelegate` :!event `SpawnEnemy`) (`self.SpawnDelay`) true))
  (bind _output_get (set `self.TimerHandle` _returnvalue))
  (`KismetSystemLibrary.K2_PauseTimerHandle` _output_get))

(event `self.ReceiveAnyDamage`
  (params (Damage :type "Float (single-precision)") (DamageType :type "DamageType Object Reference") (InstigatedBy :type "Controller Object Reference") (DamageCauser :type "Actor Object Reference"))
  (bind _output_get (set `self.SpawnerHealth` (- (`self.SpawnerHealth`) Damage)))
  (if (<= _output_get 0.0)
    (`/Game/HAN23100176/Gameplay/EnemySystem/BP_EnemyManager.SpawnerDestroyed` (`self.ManagerRef`) self)
    (`KismetSystemLibrary.Delay` 0.2)
    (`self.K2_DestroyActor`)))

(event `self.Sphere.OnComponentBeginOverlap`
  (params (OverlappedComponent :type "PrimitiveComponent Object Reference") (OtherActor :type "Actor Object Reference") (OtherComp :type "PrimitiveComponent Object Reference") (OtherBodyIndex :type Integer) (bFromSweep :type Boolean) (SweepResult :type "HitResult Structure (by ref)"))
  ;[1 1 1] Activate Spawning When Player In Range
  (if (`self.ActorHasTag` OtherActor "Player")
    (`KismetSystemLibrary.K2_UnPauseTimerHandle` (`self.TimerHandle`))))

(event `self.Sphere.OnComponentEndOverlap`
  (params (OverlappedComponent :type "PrimitiveComponent Object Reference") (OtherActor :type "Actor Object Reference") (OtherComp :type "PrimitiveComponent Object Reference") (OtherBodyIndex :type Integer))
  ;[1 1 1] Activate Spawning When Player In Range
  (if (`self.ActorHasTag` OtherActor "Player")
    (`KismetSystemLibrary.K2_PauseTimerHandle` (`self.TimerHandle`))))

(fn `UserConstructionScript`)