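; GM_EradicateVs is the game mode for a versus Eradicate match, tracking when all enemies have been killed.
; On BeginPlay it spawns a BP_EnemyManager at the world origin and initializes it with a self reference and a small enemy count.
; WinEnemiesKilled takes the winning team, prints the result, sets AllEnemiesKilled and calls CanEndGame to check for match end.
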(event `self.ReceiveBeginPlay`
  (`parent.ReceiveBeginPlay`)
  (`KismetSystemLibrary.PrintString` "GM Eradicate Versus Running")
  (`self.InitEnemyManager`))

(event `InitEnemyManager`
  (bind _returnvalue (`|SpawnActorFromClass` "/Game/HAN23100176/Gameplay/BP_EnemyManager.BP_EnemyManager_C" (`KismetMathLibrary.MakeTransform` (0.0 0.0 0.0)) "Undefined" "OverrideRootScale" null null))
  (`/Game/HAN23100176/Gameplay/BP_EnemyManager.InitEnemies` _returnvalue self 3))

(event `/Game/HAN23100176/Gameplay/BPI_WinConditions.Win_EnemiesKilled`
  (params (WinningTeam :type "/Game/HAN23100176/Gameplay/E_Teams Enum" :default "NewEnumerator0"))
  (`KismetSystemLibrary.PrintString` (`KismetStringLibrary.Concat_StrStr` (`|GetEnumeratorNameAsString` WinningTeam) " wins!"))
  (set `self.AllEnemiesKilled` true)
  (`self.CanEndGame`))

(fn `UserConstructionScript`
  (`parent.UserConstructionScript`))