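; Base game mode for local multiplayer levels, handling player setup, character spawning and the level-end screen.
; On BeginPlay it rebuilds local players from the PlayerCount URL option, tracking each PC_Gameplay through login and logout.
; Each controller possesses a colored character chosen by its PlayerType option, spawned at one hardcoded location.
; It binds to BP_LevelEndTrigger to show WBP_EndScreen with UI-only input for the first player.
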(event `self.ReceiveBeginPlay`
  (`self.SetupControllers` (`GameplayStatics.GetIntOption` (`self.OptionsString`) "PlayerCount" 1))
  (`self.SpawnCharacters`)
  (bind _returnvalue (`GameplayStatics.GetActorOfClass` "/Game/HAN23100176/Gameplay/BP_LevelEndTrigger.BP_LevelEndTrigger_C"))
  (add `/Game/HAN23100176/Gameplay/BP_LevelEndTrigger.LevelEnd` _returnvalue (`|CreateDelegate` :!event `OnLevelEnd`)))

(event `self.K2_PostLogin`
  (params (NewPlayer :type "PlayerController Object Reference"))
  (bind _aspc_gameplay (cast `/Game/HAN23100176/Gameplay/PC_Gameplay` NewPlayer))
  (`KismetArrayLibrary.Array_Add` (`self.As PC Gameplay`) _aspc_gameplay))

(event `self.K2_OnLogout`
  (params (ExitingController :type "Controller Object Reference"))
  (bind _aspc_gameplay (cast `/Game/HAN23100176/Gameplay/PC_Gameplay` ExitingController))
  (`KismetArrayLibrary.Array_RemoveItem` (`self.As PC Gameplay`) _aspc_gameplay))

(event `OnLevelEnd`
  (if true
    (bind _returnvalue (`|CreateWidget` "/Game/HAN23100176/UI/WBP_EndScreen.WBP_EndScreen_C"))
    (`UserWidget.AddToViewport` _returnvalue 0)
    (`WidgetBlueprintLibrary.SetInputMode_UIOnlyEx` (`PlayerState.GetPlayerController` (`Controller.PlayerState` (`GameplayStatics.GetPlayerControllerFromID` 0))) null)))

(fn `SetupControllers`
  (params (NumberOfPlayers :type Integer))
  (`GameplayStatics.RemovePlayer` (`GameplayStatics.GetPlayerController` 0) true)
  (for _index (range NumberOfPlayers)
    (`GameplayStatics.CreatePlayer` _index)))

(fn `SpawnCharacters`
  (for (_array_element _array_index) (`self.As PC Gameplay`)
    (bind _returnvalue (`|SpawnActorFromClass` (select `int` (- (`KismetMathLibrary.Clamp` (`GameplayStatics.GetIntOption` (`self.OptionsString`) (select `int` _array_index :`0` "Player1Type" :`1` "Player2Type" :`2` "Player3Type" :`3` "Player4Type") 1) 1 4) 1) :`0` "/Game/HAN23100176/Characters/BP_Character_Blue.BP_Character_Blue_C" :`1` "/Game/HAN23100176/Characters/BP_Character_Green.BP_Character_Green_C" :`2` "/Game/HAN23100176/Characters/BP_Character_Orange.BP_Character_Orange_C" :`3` "/Game/HAN23100176/Characters/BP_Character_Red.BP_Character_Red_C" :!type "Actor Class Reference") (`KismetMathLibrary.MakeTransform` (2000.0 1000.0 250.0)) "AdjustIfPossibleButAlwaysSpawn" "OverrideRootScale" null null))
    (`Controller.Possess` _array_element (cast `Pawn` _returnvalue :!pure true))))

(fn `UserConstructionScript`)