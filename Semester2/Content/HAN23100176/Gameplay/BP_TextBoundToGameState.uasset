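; Actor that displays the current match phase as world text through a Text Render component.
; On BeginPlay it casts the game state to GS_GameStateBase and binds to its state-changed event.
; Each change sets the text to a get-ready, begin or game-over message for the pre, in and post game phases.
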(event `self.ReceiveBeginPlay`
  (bind (_asgs_game_state_base _bsuccess) (cast `/Game/HAN23100176/Gameplay/GS_GameStateBase` (`GameplayStatics.GetGameState`) :!pure true))
  (if _bsuccess
    (add `/Game/HAN23100176/Gameplay/GS_GameStateBase.GameStateChanged` _asgs_game_state_base (delegate `StateChanged`))))

(event `StateChanged`
  (params (CurrentGameState :type "/Game/HAN23100176/Gameplay/E_GameState Enum" :default "NewEnumerator0"))
  (switch `/Game/HAN23100176/Gameplay/E_GameState` CurrentGameState
    (:`NewEnumerator1`
      (`TextRenderComponent.K2_SetText` (`self.TextRender`) "Get Ready"))
    (:`NewEnumerator2`
      (`TextRenderComponent.K2_SetText` (`self.TextRender`) "Begin"))
    (:`NewEnumerator3`
      (`TextRenderComponent.K2_SetText` (`self.TextRender`) "Game Over"))))

(fn `UserConstructionScript`)