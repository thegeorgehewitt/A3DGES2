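; Pickup manager that spawns collectible pickups, tallies them for two teams and decides the winning team.
; InitPickups spawns pickups just above the first requested number of spawn-point actors, passing itself as manager, and binds to OnPickupCollected.
; PickupCollected increments the collecting team's count and removes the pickup from the remaining list.
; Once none remain, it compares counts, allowing a draw, and reports the result through the GMRef reference.
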(event `InitPickups`
  (params (GMRef :type "GameModeBase Object Reference") (NumOfPickups :type Integer))
  (set `self.GMRef` GMRef)
  (bind _outactors (`GameplayStatics.GetAllActorsOfClass` "/Game/HAN23100176/Gameplay/BP_PickupSpawn.BP_PickupSpawn_C"))
  (for (_array_element _array_index) _outactors
    (if (< _array_index NumOfPickups)
      (bind _returnvalue (`|SpawnActorFromClass` "/Game/HAN23100176/Gameplay/BP_Pickup.BP_Pickup_C" (`KismetMathLibrary.MakeTransform` (+ (`self.K2_GetActorLocation` _array_element) (0.0 0.0 50.0))) "Undefined" "OverrideRootScale" null self null))
      (`KismetArrayLibrary.Array_Add` (`self.PickupsRemaining`) _returnvalue)))
  (add `self.OnPickupCollected` (`|CreateDelegate` :!event `PickupCollected`)))

(event `PickupCollected` :!signature `self.OnPickupCollected`
  (params (ActorRef :type "/Game/HAN23100176/Gameplay/BP_Pickup Object Reference") (Team :type "/Game/HAN23100176/Gameplay/E_Teams Enum" :default "NewEnumerator0"))
  (bind _pickupsremaining (`self.PickupsRemaining`))
  (switch `/Game/HAN23100176/Gameplay/E_Teams` Team
    (:`NewEnumerator0`
      _)
    (:`NewEnumerator1`
      (`/Engine/EditorBlueprintResources/StandardMacros.IncrementInt` (`self.TeamAPickups`)
        (:`  `
          _)))
    (:`NewEnumerator2`
      (`/Engine/EditorBlueprintResources/StandardMacros.IncrementInt` (`self.TeamBPickups`)
        (:`  `
          _))))
  (`KismetArrayLibrary.Array_RemoveItem` _pickupsremaining ActorRef)
  (if (== (`KismetArrayLibrary.Array_Length` _pickupsremaining) 0)
    (if (== (`self.TeamAPickups`) (`self.TeamBPickups`))
      (set `self.WinningTeam` "NewEnumerator0")
      (elif (> (`self.TeamAPickups`) (`self.TeamBPickups`))
        (set `self.WinningTeam` "NewEnumerator1")
        (else
          (set `self.WinningTeam` "NewEnumerator2"))))
    (message `/Game/HAN23100176/Gameplay/BPI_WinConditions.Win_Collected` (`self.GMRef`) (`self.WinningTeam`))))

(fn `UserConstructionScript`)