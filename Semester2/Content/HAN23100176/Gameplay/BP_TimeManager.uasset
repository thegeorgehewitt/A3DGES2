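; BP_TimeManager runs a one-shot countdown and notifies GMRef, likely the game mode, when time runs out.
; InitTimer starts a non-looping event timer of the given length and stores its handle.
; TimerComplete calls TimeUp on GMRef, while GetTimeElapsed reads the stored handle and returns the elapsed time rounded to hundredths of a second.
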(event `InitTimer`
  (params (TimerLength :type "Float (double-precision)") (GMRef :type "/Game/HAN23100176/Gameplay/GM_Base Object Reference"))
  (bind _returnvalue (`KismetSystemLibrary.K2_SetTimerDelegate` (delegate `TimerComplete`) TimerLength))
  (set `self.TimeHandle` _returnvalue))

(event `TimerComplete`
  (`/Game/HAN23100176/Gameplay/GM_Base.TimeUp` (stale `InitTimer` GMRef)))

(fn `GetTimeElapsed`
  (returns (TimeElapsed :type "Float (double-precision)"))
  (return (* (`KismetMathLibrary.Round` (* (`KismetSystemLibrary.K2_GetTimerElapsedTimeHandle` (`self.TimeHandle`)) 100.0)) 0.01)))

(fn `UserConstructionScript`)