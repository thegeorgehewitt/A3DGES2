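; BP_TeamsPlayerStart is a team-assigned spawn point that stores a TeamID of No Team, Team A or Team B.
; Its construction script sets a text render component's label and color to match the assigned team, giving a visual indicator of the assignment.
; A SetTeam event changes the TeamID without refreshing the label, and GetTeam returns it.
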(event `/Game/HAN23100176/Gameplay/BPI_PlayerData.SetTeam`
  (params (TeamID :type "/Game/HAN23100176/Gameplay/E_Teams Enum" :default "NewEnumerator0"))
  (set `self.TeamID` TeamID))

(fn `GetTeam`
  (returns (TeamID :type "/Game/HAN23100176/Gameplay/E_Teams Enum"))
  (return (`self.TeamID`)))

(fn `UserConstructionScript`
  (bind _teamid (`self.TeamID`))
  (switch `/Game/HAN23100176/Gameplay/E_Teams` _teamid
    (:`NewEnumerator0`
      (`TextRenderComponent.K2_SetText` (`self.TextRender`) "No Assignment"))
    (:`NewEnumerator1`
      (`TextRenderComponent.K2_SetText` (`self.TextRender`) "Team A"))
    (:`NewEnumerator2`
      (`TextRenderComponent.K2_SetText` (`self.TextRender`) "Team B")))
  (`TextRenderComponent.SetTextRenderColor` (`self.TextRender`) (select `/Game/HAN23100176/Gameplay/E_Teams` _teamid :`NewEnumerator0` (`KismetMathLibrary.LinearColor_ToRGBE` (struct :`R` 0.08981 :`G` 0.21875 :`B` 0.118967 :`A` 1.0)) :`NewEnumerator1` (`KismetMathLibrary.LinearColor_ToRGBE` (struct :`R` 0.328125 :`G` 0.190627 :`B` 0.063232 :`A` 1.0)) :`NewEnumerator2` (`KismetMathLibrary.LinearColor_ToRGBE` (struct :`R` 0.119819 :`G` 0.133758 :`B` 0.21875 :`A` 1.0)))))