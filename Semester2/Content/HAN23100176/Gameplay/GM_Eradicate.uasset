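; Game mode for an Eradicate match, which is won when a kill limit is reached.
; On BeginPlay it spawns a BP_KillLimitManager and initializes it with a reference to itself and the target kill count.
; WinEnemiesKilled takes the winning team, prints the result, sets KillLimitReached and calls CanEndGame to handle ending the match.
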(event `self.ReceiveBeginPlay`
  (`parent.ReceiveBeginPlay`)
  (`KismetSystemLibrary.PrintString` "GM_TDM Running")
  (`self.InitKillLimit`))

(event `InitKillLimit`
  (bind _returnvalue (`|SpawnActorFromClass` "/Game/HAN23100176/Gameplay/BP_KillLimitManager.BP_KillLimitManager_C" (`KismetMathLibrary.MakeTransform` (0.0 0.0 0.0)) "Undefined" "OverrideRootScale" null null))
  (`/Game/HAN23100176/Gameplay/BP_KillLimitManager.Init` _returnvalue self 3))

(event `/Game/HAN23100176/Gameplay/BPI_WinConditions.Win_EnemiesKilled`
  (params (WinningTeam :type "/Game/HAN23100176/Gameplay/E_Teams Enum" :default "NewEnumerator0"))
  (`KismetSystemLibrary.PrintString` (`KismetStringLibrary.Concat_StrStr` (`|GetEnumeratorNameAsString` WinningTeam) " wins!"))
  (set `self.KillLimitReached` true)
  (`self.CanEndGame`))

(fn `UserConstructionScript`
  (`parent.UserConstructionScript`))