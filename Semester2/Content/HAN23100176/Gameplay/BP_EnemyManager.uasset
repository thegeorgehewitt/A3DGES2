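; BP_EnemyManager runs the enemy spawner objective and decides which team wins by kill count.
; On init it spawns and initializes BP_EnemySpawners at BP_SpawnerPoints locations, up to a requested count, and binds spawner-destroyed and enemy-killed events.
; It tracks remaining spawners, live enemies and kills per team.
; Once both lists are cleared, it reports the winning team, or no team on a tie, to the game mode reference.
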(event `InitEnemySpawners`
  (params (GMRef :type "GameModeBase Object Reference") (NumOfSpawners :type Integer))
  (set `self.GMRef` GMRef)
  (bind _outactors (`GameplayStatics.GetAllActorsOfClass` "/Game/HAN23100176/Gameplay/BP_SpawnerPoints.BP_SpawnerPoints_C"))
  (for (_array_element _array_index) _outactors
    (if (< _array_index NumOfSpawners)
      (bind _returnvalue (`|SpawnActorFromClass` "/Game/HAN23100176/Gameplay/BP_EnemySpawner.BP_EnemySpawner_C" (`KismetMathLibrary.MakeTransform` (`self.K2_GetActorLocation` _array_element)) "Undefined" "OverrideRootScale" null self null))
      (`KismetArrayLibrary.Array_Add` (`self.SpawnersRemaining`) _returnvalue)
      (`/Game/HAN23100176/Gameplay/BP_EnemySpawner.InitEnemies` _returnvalue)))
  (add `self.OnSpawnerDestroyed` (`|CreateDelegate` :!event `SpawnerDestroyed`))
  (add `self.OnEnemyKilled` (`|CreateDelegate` :!event `EnemyKilled`)))

(event `EnemyKilled` :!signature `self.OnEnemyKilled`
  (params (KilledActor :type "/Game/HAN23100176/Characters/Enemy/BP_EnemyCharacter Object Reference") (Team :type "/Game/HAN23100176/Gameplay/E_Teams Enum" :default "NewEnumerator0"))
  (bind _enemiesremaining (`self.EnemiesRemaining`))
  (switch `/Game/HAN23100176/Gameplay/E_Teams` Team
    (:`NewEnumerator0`
      _)
    (:`NewEnumerator1`
      (`/Engine/EditorBlueprintResources/StandardMacros.IncrementInt` (`self.TeamAKills`)
        (:`  `
          _)))
    (:`NewEnumerator2`
      (`/Engine/EditorBlueprintResources/StandardMacros.IncrementInt` (`self.TeamBKills`)
        (:`  `
          _))))
  (`KismetArrayLibrary.Array_RemoveItem` _enemiesremaining KilledActor)
  (if (== (`KismetArrayLibrary.Array_Length` _enemiesremaining) 0)
    (set `self.EnemiesCleared` true)
    (`self.ConditionsMet`)))

(event `EnemySpawned`
  (params (SpawnedActor :type "/Game/HAN23100176/Characters/Enemy/BP_EnemyCharacter Object Reference"))
  (`KismetArrayLibrary.Array_Add` (`self.EnemiesRemaining`) SpawnedActor)
  (set `self.EnemiesCleared` false))

(event `SpawnerDestroyed` :!signature `self.OnSpawnerDestroyed`
  (params (DestroyedActor :type "/Game/HAN23100176/Gameplay/BP_EnemySpawner Object Reference"))
  (bind _spawnersremaining (`self.SpawnersRemaining`))
  (`KismetArrayLibrary.Array_RemoveItem` _spawnersremaining DestroyedActor)
  (if (== (`KismetArrayLibrary.Array_Length` _spawnersremaining) 0)
    (set `self.SpawnersCleared` true)
    (`self.ConditionsMet`)))

(event `ConditionsMet`
  (if (and (`self.SpawnersCleared`) (`self.EnemiesCleared`))
    (if (== (`self.TeamAKills`) (`self.TeamBKills`))
      (set `self.WinningTeam` "NewEnumerator0")
      (elif (> (`self.TeamAKills`) (`self.TeamBKills`))
        (set `self.WinningTeam` "NewEnumerator1")
        (else
          (set `self.WinningTeam` "NewEnumerator2"))))
    (message `/Game/HAN23100176/Gameplay/Interfaces/BPI_WinConditions.Win_EnemiesKilled` (`self.GMRef`) (`self.WinningTeam`))))

(fn `UserConstructionScript`)