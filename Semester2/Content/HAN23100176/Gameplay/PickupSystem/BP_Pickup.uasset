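; BP_Pickup is a timed pickup actor that reports its collection or expiry to a manager.
; A randomized timer set at BeginPlay limits its lifetime.
; Overlap on Sphere1 reports collection with the team from the character's PC, or a default enum value for other actors.
; Collection and despawn share cleanup that restores the manager's spawn point, deactivates both spheres and destroys the actor after a short delay.
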(event `self.ReceiveBeginPlay`
  (bind _output_get (set `self.Lifetime` (`KismetMathLibrary.RandomFloatInRange` 5.0 30.0)))
  (`KismetSystemLibrary.K2_SetTimerDelegate` (`|CreateDelegate` :!event `Despawn`) _output_get))

(event `Despawn`
  (`/Game/HAN23100176/Gameplay/PickupSystem/BP_PickupManager.PickUpDespawned` (`self.ManagerRef`) self)
  (`/Game/HAN23100176/Gameplay/PickupSystem/BP_PickupManager.RestoreSpawnPoint` (`self.ManagerRef`) (`self.SpawnPoint`) :!label _label)
  (`ActorComponent.SetActive` (`self.Sphere`) false false)
  (`ActorComponent.SetActive` (`self.Sphere1`) false false)
  (`KismetSystemLibrary.Delay` 0.2)
  (`self.K2_DestroyActor`))

(event `self.Sphere1.OnComponentBeginOverlap`
  (params (OverlappedComponent :type "PrimitiveComponent Object Reference") (OtherActor :type "Actor Object Reference") (OtherComp :type "PrimitiveComponent Object Reference") (OtherBodyIndex :type Integer) (bFromSweep :type Boolean) (SweepResult :type "HitResult Structure (by ref)"))
  (bind _asbp_third_person_character (cast `/Game/HAN23100176/Characters/Paladin/BP_ThirdPersonCharacter` OtherActor)
    (:`then`
      (bind _teamid (message `/Game/HAN23100176/Gameplay/Interfaces/BPI_PlayerData.GetTeam` (`/Game/HAN23100176/Characters/Paladin/BP_ThirdPersonCharacter.PC` _asbp_third_person_character)))
      (`/Game/HAN23100176/Gameplay/PickupSystem/BP_PickupManager.OnPickupCollected` (`self.ManagerRef`) self _teamid)
      (goto _label))
    (:`CastFailed`
      (`/Game/HAN23100176/Gameplay/PickupSystem/BP_PickupManager.OnPickupCollected` (`self.ManagerRef`) self "NewEnumerator0")
      (goto _label))))

(fn `UserConstructionScript`)