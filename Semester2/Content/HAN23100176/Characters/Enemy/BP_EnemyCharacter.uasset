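; Enemy character that chases a seen player, plays punch attacks and dies when its health runs out.
; Pawn sensing feeds an AI move-to that triggers the punch montage and sound; the overlap-based damage call is disconnected.
; Hits from unseen attackers turn it via timeline; death reports the killer's team to a manager, then destroys it after a delay.
; Game state changes toggle whether it is active.
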(event `self.ReceiveBeginPlay`
  ;[1 1 1] Set Starting Health
  (set `self.Health` (`self.MaxHealth`))
  (bind _output_get (set `self.MyGameState` (cast `/Game/HAN23100176/Gameplay/GS_GameStateBase` (`GameplayStatics.GetGameState`) :!pure true)))
  (add `/Game/HAN23100176/Gameplay/GS_GameStateBase.GameStateChanged` _output_get (`|CreateDelegate` :!event `GameStateChanged`))
  (set `self.IsActive` true))

(event `self.PawnSensing.OnSeePawn`
  (params (Pawn :type "Pawn Object Reference"))
  ;[1 1 1] Sense Player
  (if (`self.Is Dead`)
    _
    (elif (`KismetSystemLibrary.DoesImplementInterface` Pawn "/Game/HAN23100176/Gameplay/Interfaces/BPI_Killable.BPI_Killable_C")
      (bind _isdead (message `/Game/HAN23100176/Gameplay/Interfaces/BPI_Killable.CheckIsDead` Pawn))
      (if _isdead
        _
        (elif (`self.IsActive`)
          (set `self.DetectedPlayer` Pawn)
          (set `self.IsSeeingPlayer` true)
          (`self.FollowPlayer`)
          (set `self.IsSeeingPlayer` false))))))

(event `FollowPlayer`
  ;[1 1 1] Move To Player
  (if (not (`self.Is Dead`))
    (if (`self.IsActive`)
      (if (`self.IsSeeingPlayer`)
        (`|AIMoveTo` self (0.0 0.0 0.0) (`self.DetectedPlayer`) 50.0
          (:`OnSuccess`
            (if (`self.CanAttack`)
              (set `self.CanAttack` false)
              (`|PlayMontage` (`self.Mesh`) "/Game/HAN23100176/Characters/Enemy/Animations/AM_Punch.AM_Punch"
                (:`then`
                  (`self.HitPlayer`))
                (:`OnCompleted`
                  (set `self.CanAttack` true))))))
        (else
          (set `self.CanAttack` false))))))

(event `HitPlayer`
  ;[1 1 1] Hit/Damage Player
  (`KismetSystemLibrary.Delay` 0.2)
  (for _array_element (`PrimitiveComponent.GetOverlappingActors` (`self.Box`) "/Game/HAN23100176/Characters/Paladin/BP_ThirdPersonCharacter.BP_ThirdPersonCharacter_C")
    _)
  (`GameplayStatics.PlaySound2D` "/Game/HAN23100176/SFX/EnemyAttackCue.EnemyAttackCue" 1.0 1.0 0.0 null null))

(event `self.ReceiveAnyDamage`
  (params (Damage :type "Float (single-precision)") (DamageType :type "DamageType Object Reference") (InstigatedBy :type "Controller Object Reference") (DamageCauser :type "Actor Object Reference"))
  ;[1 1 1] Taking Damage/Death
  (if (not (`self.Is Dead`))
    (if (`self.IsActive`)
      (bind _output_get (set `self.Health` (- (`self.Health`) (`KismetMathLibrary.FTrunc` Damage))))
      (if (<= _output_get 0)
        (`GameplayStatics.PlaySound2D` "/Game/HAN23100176/SFX/DeathCue.DeathCue" 1.0 1.0 0.0 null null)
        (set `self.Is Dead` true)
        (set `self.IsSeeingPlayer` false)
        (set `self.CanAttack` false)
        (bind _asbp_third_person_character (cast `/Game/HAN23100176/Characters/Paladin/BP_ThirdPersonCharacter` DamageCauser)
          (:`then`
            (bind _teamid (message `/Game/HAN23100176/Gameplay/Interfaces/BPI_PlayerData.GetTeam` (`/Game/HAN23100176/Characters/Paladin/BP_ThirdPersonCharacter.PC` _asbp_third_person_character)))
            (`/Game/HAN23100176/Gameplay/EnemySystem/BP_EnemyManager.OnEnemyKilled` (`self.ManagerRef`) self _teamid))
          (:`CastFailed`
            (`/Game/HAN23100176/Gameplay/EnemySystem/BP_EnemyManager.OnEnemyKilled` (`self.ManagerRef`) self "NewEnumerator0")))
        (`KismetSystemLibrary.K2_SetTimerDelegate` (delegate `AfterDeathTimer`) 5.0)
        (else
          ;[1 1 1] If hit and not seeing player, turn to player
          (if (not (`self.IsSeeingPlayer`))
            (bind _aspawn (cast `Pawn` DamageCauser))
            (set `self.DetectedPlayer` _aspawn)
            (set `self.StartRotation` (`self.K2_GetActorRotation`))
            (bind (_direction _newtrack_0) (`Timeline|Timeline` :!label _label)
              (:`Update`
                (`self.K2_SetActorRotation` (`KismetMathLibrary.RLerp` (`self.StartRotation`) (`KismetMathLibrary.FindLookAtRotation` (`self.K2_GetActorLocation`) (`self.K2_GetActorLocation` (`self.DetectedPlayer`))) _newtrack_0 true))
                (if (`self.IsSeeingPlayer`)
                  (goto _label :!via `Stop`))))))))))

(event `AfterDeathTimer`
  ;[1 1 1] Taking Damage/Death
  (`self.K2_DestroyActor`))

(event `GameStateChanged`
  (params (CurrentGameState :type "/Game/HAN23100176/Gameplay/E_GameState Enum" :default "NewEnumerator0"))
  (switch `/Game/HAN23100176/Gameplay/E_GameState` CurrentGameState
    (:`NewEnumerator0`
      (set `self.IsActive` false :!label _label_2))
    (:`NewEnumerator1`
      (goto _label_2))
    (:`NewEnumerator2`
      (set `self.IsActive` true))
    (:`NewEnumerator3`
      (goto _label_2))))

(fn `GetIsDead`
  (returns (IsDead :type Boolean))
  (return (`self.Is Dead`)))

(fn `UserConstructionScript`)